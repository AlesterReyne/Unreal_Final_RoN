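; Base weapon Blueprint providing hitscan firing, with empty Shoot, EndShoot and SpawnSFX events.
; CreateShotTrace spends ammo, spawns a muzzle effect and line-traces from ShootArrow, damaging only the first hit.
; The hit actor's first tag selects a surface-specific impact particle, with blood for Humanoid and ceramic as default.
; It updates the owning player's HUD ammo count; an empty magazine clears CanShoot and prints a placeholder SFX message.
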(event Custom|CreateShotTrace
  (params (Range :type Float%20%28double-precision%29))
  (|RaycastTrace Range))

(event Custom|EndShoot)

(event Custom|Shoot)

(event Custom|SpawnHitParticles
  (params (Tag%20Name :type Name) (Location :type Vector) (Arrow%20Rotation :type Rotator))
  (|Particles Tag%20Name Location Arrow%20Rotation))

(event Custom|SpawnSFX)

(event EventBeginPlay)

(fn ConstructionScript)