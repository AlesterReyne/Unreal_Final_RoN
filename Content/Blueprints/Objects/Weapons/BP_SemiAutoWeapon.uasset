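; Semi-automatic weapon Blueprint that overrides the parent's Shoot event to fire one trace shot at a time, limited by fire rate.
; When CanShoot is true, Shoot clears it, runs a shot trace over Range and plays the semi-auto sound.
; It then starts a looping timer at the FireRate interval, stored in Timer, whose ResetShot event sets CanShoot back to true.
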(event Custom|ResetShot
  (Variables|Default|SetCanShoot true))

(event EventShoot
  (|CallParentFunction)
  (if (Variables|Default|GetCanShoot)
    (Variables|Default|SetCanShoot false)
    (CallFunction|CreateShotTrace (Variables|Default|GetRange))
    (CallFunction|PlayWeaponSFX (Variables|Default|GetSemiSFX))
    (bind _returnvalue (Utilities|Time|SetTimerbyEvent (delegate Custom|ResetShot) (Variables|Default|GetFireRate) true))
    (Variables|Default|SetTimer _returnvalue)))

(fn ConstructionScript
  (|CallParentFunction))