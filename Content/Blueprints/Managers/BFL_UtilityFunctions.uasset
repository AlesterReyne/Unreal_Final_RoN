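; Blueprint function library of utility lookups for BP_TargetPoint actors by name.
; GetAllTargetPointsWithName scans every BP_TargetPoint in the world and collects those whose TargetName matches the given name.
; GetRandomPointWithName builds on that list and returns one randomly chosen match, with no guard for an empty result.
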(fn GetAllTargetPointswithName
  (params (Target%20Name :type String))
  (bind _outactors (Actor|GetAllActorsOfClass 0 "/Game/Blueprints/Characters/Enemy/BP_TargetPoint.BP_TargetPoint_C"))
  (for _array_element _outactors
    (bind _asbp_target_point (Utilities|Casting|CastToBP_TargetPoint _array_element))
    (if (Utilities|Enum|Equal(Enum) Target%20Name (Variables|/Game/Blueprints/Characters/Enemy/BP_TargetPoint.BP_TargetPoint_C|GetTarget%20Name _asbp_target_point))
      (Utilities|Array|SetArrayElem (LocalVariables|GetT_Pts) (Utilities|Array|Length (LocalVariables|GetT_Pts)) _asbp_target_point true)))
  (return (LocalVariables|GetT_Pts)))

(fn GetRandomPointwithName
  (params (Name :type String))
  (bind _target_points (CallFunction|GetAllTargetPointswithName Name))
  (return (Utilities|Array|Get(acopy) _target_points (Math|Random|RandomIntegerinRange 0 (- (Utilities|Array|Length _target_points) 1)))))