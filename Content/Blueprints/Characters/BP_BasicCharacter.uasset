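; Base character Blueprint that supplies reload cancelling, aim rotation and hand sway data, apparently for a first-person or shooter rig.
; StopReload instantly stops a playing reload montage, clears IsReloading and destroys any held magazine.
; GetAimRotation converts control pitch to a signed, inverted angle and outputs a third of it as roll, suiting spreading across bones.
; GetHandSway exposes sideways move input and mouse axes.
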(event Custom|StopReload
  (bind _mesh (Variables|Character|GetMesh))
  (bind _heldmag (Variables|Default|GetHeldMag))
  (bind _returnvalue (Components|SkeletalMesh|GetAnimInstance _mesh))
  (if (Animation|Montage|MontageIsPlaying _returnvalue "/Game/Animations/Montages/AM_Reload.AM_Reload")
    (Animation|Montage|MontageStop _returnvalue 0.0 "/Game/Animations/Montages/AM_Reload.AM_Reload")
    (Variables|Animations|SetisReloading false)
    (Utilities|IsValid _heldmag
      (:Is%20Valid
        (Actor|DestroyActor _heldmag)))))

(fn ConstructionScript)

(fn GetAimRotation
  (bind _returnvalue (Pawn|GetControlRotation :!class /Script/Engine.Pawn))
  (return (Math|Rotator|MakeRotator (/ (Math|Float|SelectFloat (- 3.6e+02 (.pitch _returnvalue)) (* (.pitch _returnvalue) -1.0) (> (.pitch _returnvalue) 1.8e+02)) 3.0) 0.0 0.0)))

(fn GetHandSway
  (return (.x (Input|EnhancedActionValues|GetIA_Move)) (Class|Actor|GetInputAxisKeyValue) (Class|Actor|GetInputAxisKeyValue)))