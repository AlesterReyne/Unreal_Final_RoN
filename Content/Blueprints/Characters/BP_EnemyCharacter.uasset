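; Enemy AI character that patrols, spots the player, investigates and enters combat, with health and a socket-attached weapon.
; Tick runs an enum state machine that sets walk speed and moves between named patrol points with AIMoveTo.
; Vision combines range, line trace and dot-product cone; sustained sighting triggers investigation, close sighting triggers combat.
; Damage triggers combat, cover-seeking at low health, or death; combat and cover behaviours are placeholder prints.
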(event Custom|OnRequestInvestigatePosition_Event
  ;[0.15 0.15 0.15 0.5] Events
  (AI|AIMoveTo (Class|PawnMovementComponent|GetPawnOwner (Variables|Character|GetCharacterMovement)) (Variables|Enemy|Behavior|GetInvestigationPosition) 0 5.0 false))

(event EventBeginPlay
  ;[0.15 0.15 0.15 0.5] Errors
  (if (<= (Variables|Enemy|Distances|GetMaxVisionDistance) (Variables|Enemy|Distances|GetDistanceToSeePlayerAndInitiateCombat))
    (Development|PrintString "ERROR : ENEMY VISION INVALID")
    (else
      ;[0.15 0.15 0.15 0.5] Set Up a Weapon
      (bind _returnvalue (Game|SpawnActorfromClass (Variables|Enemy|Behavior|GetWeaponType) (Transformation|GetActorTransform) "Undefined" "MultiplyWithRoot" 0 0))
      (bind _output_get (Variables|Default|SetCurrentWeapon _returnvalue))
      (Transformation|AttachComponentToComponent _output_get (Variables|Character|GetMesh) "Rifle_Socket" "SnapToTarget" "SnapToTarget" "SnapToTarget" true)
      ;[0.15 0.15 0.15 0.5] Set Default State
      (Variables|Enemy|Behavior|SetCurrentState "NewEnumerator2")
      ;[0.15 0.15 0.15 0.5] Events
      (EventDispatchers|BindEventtoOnRequestInvestigatePosition (delegate Custom|OnRequestInvestigatePosition_Event)))))

(event EventTick
  (params (DeltaSeconds :type Float%20%28single-precision%29))
  (Variables|Enemy|Timers|SetCurrentDeltaTime DeltaSeconds)
  (Development|PrintString (Utilities|String|Append "Current State : " (Utilities|String|EnumtoString (Variables|Enemy|Behavior|GetCurrentState))) true true "(R=0.000000,G=0.660000,B=1.000000,A=1.000000)" 2.0 "State")
  (switch Utilities|FlowControl|Switch|SwitchonE_EnemyState (Variables|Enemy|Behavior|GetCurrentState)
    (:NewEnumerator2
      ;[0.15 0.15 0.15 0.5] Idle - Wait A Couple of Seconds
      ;;[0.15 0.15 0.15 0.5] Set Speed
      (Variables|/Script/Engine.CharacterMovementComponent|SetMaxWalkSpeed (Variables|Character|GetCharacterMovement) (Variables|Enemy|Speeds|GetDefaultSpeed))
      ;;[0.15 0.15 0.15 0.5] Check For Player While Idling
      (bind _isplayerinvision (CallFunction|CheckPlayerinVision))
      (if _isplayerinvision
        (CallFunction|BeginInvestigatingPlayerPosition)
        (Variables|Enemy|Timers|SetTime%20Idling 0.0 :!label _label)
        (else
          (bind _isengagedincombat (CallFunction|CheckEngageCombat))
          (if _isengagedincombat
            (goto _label)
            (else
              ;;[0.15 0.15 0.15 0.5] Increment Time Idling
              (Variables|Enemy|Timers|SetTime%20Idling (+ (Variables|Enemy|Timers|GetTime%20Idling) (Variables|Enemy|Timers|GetCurrentDeltaTime)))
              ;;[0.15 0.15 0.15 0.5] Switch To Patrol If Idled Enough
              (if (>= (Variables|Enemy|Timers|GetTime%20Idling) (Variables|Enemy|Timers|GetTime%20To%20Stay%20Idle))
                (Variables|Enemy|Timers|SetTime%20Idling 0.0)
                (Variables|Enemy|Behavior|SetCurrentState "NewEnumerator0")
                (CallFunction|ChooseNextPatrolTarget)
                (AI|AIMoveTo (Class|PawnMovementComponent|GetPawnOwner (Variables|Character|GetCharacterMovement)) "0, 0, 0" (Variables|Enemy|Behavior|GetCurrentPatrolPoint) 5.0 false)))))))
    (:NewEnumerator0
      ;[0.15 0.15 0.15 0.5] Patrol - Navigate to the target position
      ;;[0.15 0.15 0.15 0.5] Set Speed
      (Variables|/Script/Engine.CharacterMovementComponent|SetMaxWalkSpeed (Variables|Character|GetCharacterMovement) (Variables|Enemy|Speeds|GetDefaultSpeed))
      ;;[0.15 0.15 0.15 0.5] Check For Player While Patrolling
      (bind _isplayerinvision_2 (CallFunction|CheckPlayerinVision))
      (if _isplayerinvision_2
        (CallFunction|BeginInvestigatingPlayerPosition)
        (else
          (bind _isengagedincombat_2 (CallFunction|CheckEngageCombat))
          (if (not _isengagedincombat_2)
            ;;[0.15 0.15 0.15 0.5] Check If Reached Target
            (if (<= (Transformation|GetDistanceTo (Variables|Enemy|Behavior|GetCurrentPatrolPoint)) (Variables|Enemy|Distances|GetDistanceToConsiderReached))
              ;;[0.15 0.15 0.15 0.5] Switch To Idle
              (Variables|Enemy|Behavior|SetCurrentState "NewEnumerator2")
              (Variables|Enemy|Timers|SetTime%20Idling 0.0)
              (Components|Movement|StopMovementImmediately (Variables|Character|GetCharacterMovement)))))))
    (:NewEnumerator1
      ;[0.15 0.15 0.15 0.5] Investigate - Check position where player was spotted
      ;;[0.15 0.15 0.15 0.5] Set Speed
      (Variables|/Script/Engine.CharacterMovementComponent|SetMaxWalkSpeed (Variables|Character|GetCharacterMovement) (Variables|Enemy|Speeds|GetDefaultSpeed))
      ;;[0.15 0.15 0.15 0.5] Check Player To Engage In Combat
      (bind _isplayerinvision_3 (CallFunction|CheckPlayerinVision))
      (if _isplayerinvision_3
        (CallFunction|BeginInvestigatingPlayerPosition)
        (bind _isengagedincombat_3 (CallFunction|CheckEngageCombat))
        (if (not _isengagedincombat_3)
          ;;[0.15 0.15 0.15 0.5] Check If Reached Target
          (if (<= (Math|Vector|Distance(Vector) (Transformation|GetActorLocation) (Variables|Enemy|Behavior|GetInvestigationPosition)) (Variables|Enemy|Distances|GetDistanceToConsiderReached))
            ;;[0.15 0.15 0.15 0.5] Switch To Idle
            (Variables|Enemy|Behavior|SetCurrentState "NewEnumerator2" :!label _label_2)
            (Variables|Enemy|Timers|SetTime%20Idling 0.0)))
        (else
          (bind _isengagedincombat_4 (CallFunction|CheckEngageCombat))
          (if (not _isengagedincombat_4)
            (bind _output_get (Variables|Enemy|Timers|SetCurrentTimeStayingBeforeInvestigating (- (Variables|Enemy|Timers|GetCurrentTimeStayingBeforeInvestigating) (Variables|Enemy|Timers|GetCurrentDeltaTime))))
            (if (<= _output_get 0.0)
              (Variables|Enemy|Timers|SetCurrentTimeStayingBeforeInvestigating 0.0)
              (goto _label_2))))))
    (:NewEnumerator3
      ;[0.15 0.15 0.15 0.5] Combat - Shoot Player and stuff
      ;;[0.15 0.15 0.15 0.5] Set Speed
      (Variables|/Script/Engine.CharacterMovementComponent|SetMaxWalkSpeed (Variables|Character|GetCharacterMovement) (Variables|Enemy|Speeds|GetCombatSpeed))
      (bind _isplayerinvision_4 (CallFunction|CheckPlayerinVision))
      (if _isplayerinvision_4
        ;;[0.15 0.15 0.15 0.5] Move Slowly Towards Player And Shoot
        (Development|PrintString "Hello")
        (else
          ;;[0.15 0.15 0.15 0.5] Comment
          (Development|PrintString "Hello"))))
    (:NewEnumerator4
      ;[0.15 0.15 0.15 0.5] Move Towards a Cover
      ;;[0.15 0.15 0.15 0.5] Set Speed
      (Variables|/Script/Engine.CharacterMovementComponent|SetMaxWalkSpeed (Variables|Character|GetCharacterMovement) (Variables|Enemy|Speeds|GetRunSpeed))
      (Development|PrintString "Hello"))
    (:NewEnumerator5
      ;[0.15 0.15 0.15 0.5] Hide Behind A Cover
      (Development|PrintString "Hello"))))

(event Game|Damage|EventAnyDamage
  (params (Damage :type Float%20%28single-precision%29) (DamageType :type Damage%20Type%20Object%20Reference) (InstigatedBy :type Controller%20Object%20Reference) (DamageCauser :type Actor%20Object%20Reference))
  ;[0.15 0.15 0.15 0.5] Damage System
  (bind _output_get (Variables|Default|SetHealth (- (Variables|Default|GetHealth) Damage)))
  (if (<= _output_get 0.0)
    (Actor|DestroyActor)
    (Actor|DestroyActor (stale EventBeginPlay _output_get))
    (else
      ;[0.15 0.15 0.15 0.5] Enemy Logic When Hit
      (if (<= (Variables|Default|GetHealth) (Variables|Enemy|Behavior|GetHealthToCover))
        (switch Utilities|FlowControl|Switch|SwitchonE_EnemyState (Variables|Enemy|Behavior|GetCurrentState)
          (:NewEnumerator2
            _)
          (:NewEnumerator0
            _)
          (:NewEnumerator1
            _)
          (:NewEnumerator3
            _))
        (Variables|Enemy|Behavior|SetCurrentState "NewEnumerator4")
        (Development|PrintString "Move Towards New Cover")
        (else
          (Variables|Enemy|Behavior|SetCurrentState "NewEnumerator3")
          (Development|PrintString "Initiate Combat"))))))

(fn ConstructionScript
  (|CallParentFunction))

(fn CheckPlayerinVision
  (bind _returnvalue (Game|Player|GetPlayerPawn 0))
  (bind _enemyvisionangledegrees (Variables|Enemy|Distances|GetEnemyVisionAngleDegrees))
  (LocalVariables|SetPlayerPosition (Transformation|GetActorLocation _returnvalue))
  ;[0.15 0.15 0.15 0.5] If Player In Cone Vision - Switch State to Investigate
  (Class|KismetSystemLibrary|DrawDebugConeinDegrees (Transformation|GetWorldLocation (Variables|Components|GetHeadPosition)) (Math|Vector|GetRightVector (Variables|Character|GetMesh)) (Variables|Enemy|Distances|GetMaxVisionDistance) _enemyvisionangledegrees _enemyvisionangledegrees 12 "(R=1.000000,G=1.000000,B=1.000000,A=1.000000)" 0.0 0.0 "World")
  ;;[0.15 0.15 0.15 0.5] Comment
  (if (>= (Transformation|GetDistanceTo _returnvalue) (Variables|Enemy|Distances|GetMaxVisionDistance))
    (return false)
    (else
      (bind (_outhits _returnvalue_2) (Class|KismetSystemLibrary|LineTraceMultiforObjects (Transformation|GetWorldLocation (Variables|Components|GetHeadPosition)) (LocalVariables|GetPlayerPosition) (Utilities|Array|MakeArray "ObjectTypeQuery3" "ObjectTypeQuery1" "ObjectTypeQuery2" "ObjectTypeQuery4") false 0 "None" true))
      (if _returnvalue_2
        (bind _array_element (Utilities|Array|ForEachLoopwithBreak _outhits)
          (:LoopBody
            (Utilities|Casting|CastToBP_PlayerCharacter (.HitActor (Collision|BreakHitResult _array_element))
              (:then
                (return (>= (Math|Vector|DotProduct (Math|Vector|GetRightVector (Variables|Character|GetMesh)) (Math|Vector|Normalize (- (LocalVariables|GetPlayerPosition) (Transformation|GetActorLocation)))) (Math|Trig|Cos(Degrees) (Variables|Enemy|Distances|GetEnemyVisionAngleDegrees)))))
              (:CastFailed
                (return false)))))))))

(fn CheckEngageCombat
  (bind _returnvalue (Game|Player|GetPlayerPawn 0))
  (bind _returnvalue_2 (Transformation|GetDistanceTo _returnvalue))
  ;[0.15 0.15 0.15 0.5] Check Whether To Consider Player Visible Enough - Switch State to Combat
  (bind _isplayerinvision (CallFunction|CheckPlayerinVision))
  (if (and _isplayerinvision (<= _returnvalue_2 (Variables|Enemy|Distances|GetDistanceToSeePlayerAndInitiateCombat)))
    (Variables|Enemy|Behavior|SetCurrentState "NewEnumerator3")
    (return true)
    (else
      (Development|PrintString (Utilities|String|ToString(Float) _returnvalue_2))
      (return false))))

(fn ChooseNextPatrolTarget
  (LocalVariables|SetDidFindFlag false)
  (while (!= (LocalVariables|GetDidFindFlag) true)
    (bind _target_points (CallFunction|GetAllTargetPointswithName (Variables|Enemy|Behavior|GetPatrolPointName)))
    (if (<= (Utilities|Array|Length _target_points) 1)
      (LocalVariables|SetDidFindFlag true)
      (Development|PrintString "Invalid Amount of Patrol Points In level (<=1)")
      (else
        (Utilities|IsValid (Utilities|Array|Get(acopy) _target_points (Math|Random|RandomIntegerinRange 0 (- (Utilities|Array|Length _target_points) 1)))
          (:Is%20Valid
            (if (not (== (Utilities|Array|Get(acopy) _target_points (Math|Random|RandomIntegerinRange 0 (- (Utilities|Array|Length _target_points) 1))) (Variables|Enemy|Behavior|GetCurrentPatrolPoint)))
              (LocalVariables|SetDidFindFlag true)
              (Variables|Enemy|Behavior|SetCurrentPatrolPoint (Utilities|Array|Get(acopy) _target_points (Math|Random|RandomIntegerinRange 0 (- (Utilities|Array|Length _target_points) 1)))))))))))

(fn BeginInvestigatingPlayerPosition
  ;[0.15 0.15 0.15 0.5] Begin Investigating
  (if (Utilities|Enum|NotEqual(Enum) (Variables|Enemy|Behavior|GetCurrentState) (Utilities|Enum|LiteralenumE_EnemyState "NewEnumerator1"))
    (Variables|Enemy|Behavior|SetCurrentState "NewEnumerator1")
    (Variables|Enemy|Behavior|SetInvestigationPosition (Transformation|GetActorLocation (Game|Player|GetPlayerPawn 0)))
    (Development|PrintString "Player Spotted SFX" true true "(R=0.000000,G=0.660000,B=1.000000,A=1.000000)" 2.0 "TODO4")
    (Development|PrintString "Rotate Towards Player" true true "(R=0.000000,G=0.660000,B=1.000000,A=1.000000)" 2.0 "TODO5")
    (Variables|Enemy|Timers|SetCurrentTimeStayingBeforeInvestigating 0.0)
    (else
      (bind _output_get (Variables|Enemy|Timers|SetCurrentTimeStayingBeforeInvestigating (+ (Variables|Enemy|Timers|GetCurrentTimeStayingBeforeInvestigating) (Variables|Enemy|Timers|GetCurrentDeltaTime))))
      (if (>= _output_get (Variables|Enemy|Timers|GetTimeToStayBeforeInvestigating))
        (Default|CallOnRequestInvestigatePosition)))))